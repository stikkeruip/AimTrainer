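; Game state Blueprint for a tracking game, handling level restart, the menu-to-play transition, the match timer and game over.
; RemoveMenu runs on authority: it clears menu actors, spawns a movement locker per player at offset positions and, if a course is selected, spawns the tracking course.
; CreateArray then caches tracking destinations, spawns the tracking AI and disables tick, which CheckTargetSelected toggles by target selection.
; Helper functions accumulate the timer and set GameOver once the duration is reached.
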(event EventRestartGame
  (bind _returnvalue (Game|GetCurrentLevelName true))
  (Game|OpenLevel(byName) (Utilities|String|StringToName _returnvalue))
  (Input|SetInputModeGameOnly (Game|GetPlayerController 0)))

(event EventCheckTargetSelected
  (Actor|Tick|SetActorTickEnabled (not (== (Variables|Default|GetSelectedTarget) 0))))

(event EventRemoveMenu
  (bind _returnvalue (Class|GameplayStatics|GetNumPlayerControllers))
  (Networking|SwitchHasAuthority
    (:Authority
      (Utilities|FlowControl|Sequence
        (:then_0
          (bind _returnvalue_2 (Actor|GetActorOfClass "/Game/Menu/BP_InteractiveMenu.BP_InteractiveMenu_C"))
          (Actor|DestroyActor _returnvalue_2)
          (bind _outactors (Actor|GetAllActorsOfClass "/Script/AimTrainer.MenuButton"))
          (for _array_element _outactors
            (Actor|DestroyActor _array_element)))
        (:then_1
          (Variables|Default|SetNumPlayers _returnvalue)
          (for _index (range 1 _returnvalue)
            (Game|SpawnActorfromClass "/Game/Targets/BP_MovementLocker.BP_MovementLocker_C" (Math|Transform|MakeTransform (- (Variables|Default|GetInitialLocation) (* (Variables|Default|GetOffsetLocation) _index)) "0, 0, 0" "0.750000,0.750000,0.750000") "Undefined" 0 0)))
        (:then_2
          (if (Variables|Default|GetbIsCourseSelected)
            (Game|SpawnActorfromClass "/Game/Targets/BP_TrackingCourse.BP_TrackingCourse_C" (Math|Transform|MakeTransform "1060.000000,1160.000000,405.000000" "0, 0, 0" "1.000000,1.000000,1.000000") "Undefined" 0 0)
            (CallFunction|CreateArray)))))))

(fn ConstructionScript)

(fn CreateArray
  (bind _outactors (Actor|GetAllActorsOfClass "/Game/Targets/BP_TrackingDestinations.BP_TrackingDestinations_C"))
  (Variables|Default|SetAllDestinations _outactors)
  (Game|SpawnActorfromClass "/Game/Characters/TrackingAI.TrackingAI_C" (Math|Transform|MakeTransform "2130.000000,1200.000000,88.000000" "0,-180.000000, 0" "1.000000,1.000000,1.000000") "Undefined" 0 0)
  (Actor|Tick|SetActorTickEnabled false))

(fn SetGameTime
  (params (DeltaTime :type Float%20%28double-precision%29))
  (bind _output_get (Variables|Default|SetTimer (+ DeltaTime (Variables|Default|GetTimer))))
  (return (Utilities|Text|ToText(Float) _output_get "HalfToEven" false true 1 324 2 2)))

(fn IsGameEnded
  (if (>= (Variables|Default|GetTimer) (Variables|Default|GetGameDurationML))
    (Class|ATGameState|SetCurrentGameState "GameOver")))