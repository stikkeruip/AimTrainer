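; Base gun Blueprint that handles the effect and damage of a single shot.
; GunShot spawns a scaled-down explosion particle at the skeletal mesh's Muzzle socket as a muzzle flash.
; It takes the hit actor as input, with no trace of its own, and prints that actor's name when valid.
; Actors implementing the BPI_Health interface then receive the Damage value through an interface message.
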(fn ConstructionScript)

(fn GunShot
  (params (HitActor :type Actor%20Object%20Reference))
  (bind _skeletalmeshcomponent (Variables|Default|GetSkeletalMeshComponent))
  (Utilities|FlowControl|Sequence
    (:then_0
      (Effects|SpawnEmitteratLocation "/Game/Shit/StarterContent/Particles/P_Explosion.P_Explosion" (Transformation|GetSocketLocation _skeletalmeshcomponent "Muzzle") (Transformation|GetSocketRotation _skeletalmeshcomponent "None") "0.100000,0.100000,0.100000"))
    (:then_1
      (if (Utilities|IsValid HitActor)
        (Development|PrintString (Utilities|GetDisplayName HitActor))
        (bind _asbpi_health (Utilities|Casting|CastToBPI_Health HitActor))
        (Class|BPIHealth|BlueprintInteract(Message) (Utilities|ToObject(Interface) _asbpi_health) (Variables|Default|GetDamage))))))