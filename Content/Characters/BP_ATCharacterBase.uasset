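; BP_ATCharacterBase is a base character Blueprint that equips a gun and forwards shot events to it.
; On BeginPlay it spawns a GunBase_BP, stores it as GunBaseRef, and snaps it to the mesh's GunSocket.
; It also snaps the camera component to the mesh's Camera socket.
; The GunShot event casts the stored reference and calls the gun's GunShot, passing HitActor, which this graph never sets.
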(event EventBeginPlay
  (bind _mesh (Variables|Character|GetMesh))
  (bind _returnvalue (Game|SpawnActorfromClass "/Game/NewFolder/GunBase_BP.GunBase_BP_C" (Transformation|GetSocketTransform _mesh "GunSocket" "RTS_World") "Undefined" 0 0))
  (bind _output_get (Variables|Default|SetGunBaseRef _returnvalue))
  (Transformation|AttachComponentToComponent _output_get _mesh "GunSocket" "SnapToTarget" "SnapToTarget" "SnapToTarget" true)
  (Transformation|AttachComponentToComponent (Variables|Default|GetCameraComponent) _mesh "Camera" "SnapToTarget" "SnapToTarget" "SnapToTarget" true))

(event EventGunShot
  (bind _asgun_base_bp (Utilities|Casting|CastToGunBase_BP (Variables|Default|GetGunBaseRef)))
  (Default|GunShot _asgun_base_bp (Variables|Default|GetHitActor)))

(fn ConstructionScript)