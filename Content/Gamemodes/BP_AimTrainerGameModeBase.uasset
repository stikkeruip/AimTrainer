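; Game mode for an aim trainer that swaps the interactive menu for a tracking course.
; RemoveMenu destroys the menu and its buttons, raises the movement locker, then spawns BP_TrackingCourse if a course is selected.
; CreateArray then caches every tracking destination actor, spawns the TrackingAI at a fixed transform and disables the game mode's own tick.
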(fn ConstructionScript)

(fn CreateArray
  (bind _outactors (Actor|GetAllActorsOfClass "/Game/NewFolder/BP_TrackingDestinations.BP_TrackingDestinations_C"))
  (Variables|Default|SetAllDestinations _outactors)
  (Game|SpawnActorfromClass "/Game/Characters/TrackingAI.TrackingAI_C" (Math|Transform|MakeTransform "2130.000000,1200.000000,88.000000" "0,-180.000000, 0" "1.000000,1.000000,1.000000") "Undefined" 0 0)
  (Actor|Tick|SetActorTickEnabled false))

(fn RemoveMenu
  (Utilities|FlowControl|Sequence
    (:then_0
      (bind _returnvalue (Actor|GetActorOfClass "/Game/NewFolder/BP_InteractiveMenu.BP_InteractiveMenu_C"))
      (Actor|DestroyActor _returnvalue)
      (bind _outactors (Actor|GetAllActorsOfClass "/Script/AimTrainer.MenuButton"))
      (for _array_element _outactors
        (Actor|DestroyActor _array_element)))
    (:then_1
      (bind _returnvalue_2 (Actor|GetActorOfClass "/Game/NewFolder/BP_MovementLocker.BP_MovementLocker_C"))
      (Transformation|SetActorLocation _returnvalue_2 (+ (Transformation|GetActorLocation _returnvalue_2) "0,0,30.000000") false false))
    (:then_2
      (if (Variables|Default|GetbIsCourseSelected)
        (Game|SpawnActorfromClass "/Game/NewFolder/BP_TrackingCourse.BP_TrackingCourse_C" (Math|Transform|MakeTransform "1060.000000,1160.000000,405.000000" "0, 0, 0" "1.000000,1.000000,1.000000") "Undefined" 0 0)
        (CallFunction|CreateArray)))))